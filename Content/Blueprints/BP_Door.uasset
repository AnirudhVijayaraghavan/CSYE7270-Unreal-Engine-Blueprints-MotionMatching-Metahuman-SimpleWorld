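; BP_Door is an interactable door that toggles open and closed when its Interact event fires.
; A DoorOpen flag selects playing or reversing a timeline, whose DoorAngle track drives the door mesh's relative yaw.
; An interaction box adds a prompt widget, created at BeginPlay, to the viewport while the player character overlaps it and removes it on exit.
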(event `/Game/Blueprints/BPI_Interact.Interact`
  (if (not (`self.DoorOpen?`))
    (set `self.DoorOpen?` true)
    (bind (_direction _door_angle) (`Timeline|OpenClose Timeline` :!label _label)
      (:`Update`
        (`SceneComponent.K2_SetRelativeRotation` (`self.Door`) (`KismetMathLibrary.MakeRotator` 0.0 0.0 _door_angle) false false)))
    (else
      (set `self.DoorOpen?` false)
      (goto _label :!via `Reverse`))))

(event `self.ReceiveBeginPlay`
  (bind _returnvalue (`|CreateWidget` "/Game/Blueprints/P_Interact.P_Interact_C"))
  (set `self.Interact Prompt` _returnvalue))

(event `self.InteractionBox.OnComponentBeginOverlap`
  (params (OverlappedComponent :type "PrimitiveComponent Object Reference") (OtherActor :type "Actor Object Reference") (OtherComp :type "PrimitiveComponent Object Reference") (OtherBodyIndex :type Integer) (bFromSweep :type Boolean) (SweepResult :type "HitResult Structure (by ref)"))
  (if (== OtherActor (`GameplayStatics.GetPlayerCharacter` 0))
    (`UserWidget.AddToViewport` (`self.Interact Prompt`) 0)))

(event `self.InteractionBox.OnComponentEndOverlap`
  (params (OverlappedComponent :type "PrimitiveComponent Object Reference") (OtherActor :type "Actor Object Reference") (OtherComp :type "PrimitiveComponent Object Reference") (OtherBodyIndex :type Integer))
  (if (== (`GameplayStatics.GetPlayerCharacter` 0) OtherActor)
    (`Widget.RemoveFromParent` (`self.Interact Prompt`))))

(fn `UserConstructionScript`
  (`parent.UserConstructionScript`))