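; BP_DoorTeleport is an interactable door that also teleports the player character.
; Interact toggles DoorOpen and plays or reverses a timeline that drives the door's yaw.
; Independently of the door state, overlapping InteractionBox moves a BP_MHCharacter to TpPos, with location converted from actor-local to world space and rotation applied as stored.
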(event `self.Interact`
  (if (not (`self.DoorOpen?`))
    (set `self.DoorOpen?` true)
    (bind (_direction _door_angle) (`Timeline|OpenClose Timeline` :!label _label)
      (:`Update`
        (`SceneComponent.K2_SetRelativeRotation` (`self.Door`) (`KismetMathLibrary.MakeRotator` 0.0 0.0 _door_angle) false false)))
    (else
      (set `self.DoorOpen?` false)
      (goto _label :!via `Reverse`))))

(event `self.InteractionBox.OnComponentBeginOverlap`
  (params (OverlappedComponent :type "PrimitiveComponent Object Reference") (OtherActor :type "Actor Object Reference") (OtherComp :type "PrimitiveComponent Object Reference") (OtherBodyIndex :type Integer) (bFromSweep :type Boolean) (SweepResult :type "HitResult Structure (by ref)"))
  (bind (_tp_pos_location _tp_pos_rotation) (`KismetMathLibrary.BreakTransform` (`self.tp pos`)))
  (bind _asbp_mhcharacter (cast `/Game/ThirdPerson/Blueprints/BP_MHCharacter` OtherActor))
  (`self.K2_SetActorLocationAndRotation` _asbp_mhcharacter (`KismetMathLibrary.TransformLocation` (`self.GetTransform`) _tp_pos_location) _tp_pos_rotation false false))

(fn `UserConstructionScript`
  (`parent.UserConstructionScript`))